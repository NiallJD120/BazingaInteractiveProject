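; Player Blueprint that flies by driving its capsule's physics velocity from a throttle, starting at half of MaxThrust.
; Thrust axis input eases Thrust through interpolation, using a different Lerp while HyperSpeed is held, then sets forward velocity along the capsule.
; Tick applies forward plus vertical velocity, though the below-GravityThreshold vertical term currently evaluates to zero.
; Move Up / Down input is empty, with torque and offset nodes left disconnected.
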(event EventBeginPlay
  (Variables|Default|SetThrust (/ (Variables|Default|GetMaxThrust) 2.0)))

(event EventTick
  (params (DeltaSeconds :type Float%20%28single-precision%29))
  (bind _capsulecomponent (Variables|Collision|GetCapsuleComponent))
  (Utilities|FlowControl|Sequence
    (:then_0
      (if (< (Math|Vector|VectorLength (Variables|Default|GetForwardVelocity)) (Variables|Default|GetGravityThreshold))
        (Variables|Default|SetUpwards%20Velocity (* (Math|Float|Lerp 0.0 0.0 (- (Math|Vector|VectorLength (Variables|Default|GetForwardVelocity)) (Variables|Default|GetGravityThreshold))) (Math|Vector|UnrotateVector (Math|Vector|GetUpVector _capsulecomponent) (Transformation|GetWorldRotation _capsulecomponent))))
        (else
          (Variables|Default|SetUpwards%20Velocity (Math|Interpolation|VInterpTo (Variables|Default|GetUpwards%20Velocity) "0, 0, 0" (Utilities|Time|GetWorldDeltaSeconds) 2e+01)))))
    (:then_1
      (Physics|SetPhysicsLinearVelocity (Variables|Collision|GetCapsuleComponent) (+ (Variables|Default|GetForwardVelocity) (Variables|Default|GetUpwards%20Velocity)) false "None"))))

(event Input|ActionEvents|InputActionHyperSpeed
  (params (Key :type Key%20Structure :default "None"))
  (:Pressed
    (bind _output_get (Variables|Default|SetHyperSpeed true)))
  (:Released
    (Variables|Default|SetHyperSpeed false)))

(event Input|AxisEvents|InputAxisMoveUp/Down
  (params (AxisValue :type Float%20%28single-precision%29)))

(event Input|AxisEvents|InputAxisThrust
  (params (AxisValue :type Float%20%28single-precision%29))
  (Utilities|FlowControl|Sequence
    (:then_0
      (if (stale Input|ActionEvents|InputActionHyperSpeed _output_get)
        (if (not (Math|Float|NearlyEqual(Float) AxisValue 0.0 0.1))
          (Variables|Default|SetThrust (Math|Interpolation|FInterpTo (Variables|Default|GetThrust) (Math|Float|Lerp 0.0 (Variables|Default|GetThrust) (/ (+ AxisValue 1.0) 0.1)) (Utilities|Time|GetWorldDeltaSeconds) 0.5)))
        (elif (not (Math|Float|NearlyEqual(Float) AxisValue 0.0 0.1))
          (Variables|Default|SetThrust (Math|Interpolation|FInterpTo (Variables|Default|GetThrust) (Math|Float|Lerp (Variables|Default|GetThrust) 0.0 (/ (+ AxisValue 1.0) 2.0)) (Utilities|Time|GetWorldDeltaSeconds) 0.5)))))
    (:then_1
      (Variables|Default|SetForwardVelocity (* (Math|Vector|GetForwardVector (Variables|Collision|GetCapsuleComponent)) (Variables|Default|GetThrust))))))

(fn ConstructionScript)